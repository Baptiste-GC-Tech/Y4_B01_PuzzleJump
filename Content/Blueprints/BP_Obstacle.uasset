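; BP_Obstacle is an obstacle that endlessly shuttles between its starting location and a Destination offset from it.
; At BeginPlay it converts the offset to a world position and scales the Go and Return timelines by TravelDuration.
; Move waits, plays Go, waits again, plays Return, then calls itself to repeat.
; Timeline updates lerp the actor's location without sweeping for collisions.
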(event `self.ReceiveBeginPlay`
  (bind _returnvalue (/ 1.0 (`self.TravelDuration`)))
  (bind _output_get (set `self.Origin` (`self.K2_GetActorLocation`)))
  (set `self.Destination` (+ _output_get (`self.Destination`)))
  (`TimelineComponent.SetPlayRate` (`self.Go`) _returnvalue)
  (`TimelineComponent.SetPlayRate` (`self.Return`) _returnvalue)
  (`self.Move`))

(event `Move`
  (`KismetSystemLibrary.Delay` (`self.Wait`))
  (bind (_direction _travel) (`Timeline|Go` :!via `PlayFromStart`)
    (:`Update`
      (`self.K2_SetActorLocation` (`KismetMathLibrary.VLerp` (`self.Origin`) (`self.Destination`) _travel)))
    (:`Finished`
      (`KismetSystemLibrary.Delay` (`self.Wait`))
      (bind (_direction_2 _travel_2) (`Timeline|Return` :!via `PlayFromStart`)
        (:`Update`
          (`self.K2_SetActorLocation` (`KismetMathLibrary.VLerp` (`self.Destination`) (`self.Origin`) _travel_2)))
        (:`Finished`
          (`self.Move`))))))

(fn `UserConstructionScript`)