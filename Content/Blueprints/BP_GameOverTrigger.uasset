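; BP_GameOverTrigger is an overlap trigger that ends the game as a win or loss, based on its BoxType, when the third-person character enters.
; It flags every trigger instance as game over, disables character input and shows the cursor.
; Win blends the view to a CameraActor; Lose calls Death, detaches the follow camera and plays a sound.
; Both outcomes display WBP_GameOverScreen with their own result text.
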(event `self.ReceiveActorBeginOverlap`
  (params (OtherActor :type "Actor Object Reference"))
  (bind _returnvalue (`GameplayStatics.GetPlayerController` 0))
  (bind _returnvalue_2 (`GameplayStatics.GetPlayerController` 0))
  (bind _returnvalue_3 (`GameplayStatics.GetPlayerController` 0))
  (bind _asbp_third_person_character (cast `/Game/ThirdPerson/Blueprints/BP_ThirdPersonCharacter` OtherActor))
  (if (`self.GameIsOver`)
    (`KismetSystemLibrary.PrintText` "Game is over")
    (else
      (bind _outactors (`GameplayStatics.GetAllActorsOfClass` "BP_GameOverTrigger_C"))
      (for _array_element _outactors
        (set `/Game/Blueprints/BP_GameOverTrigger.GameIsOver` true _array_element))
      (`self.DisableInput` _asbp_third_person_character _returnvalue)
      (set `PlayerController.bShowMouseCursor` true _returnvalue)
      (switch `/Game/Blueprints/ETriggerType` (`self.BoxType`)
        (:`NewEnumerator0`
          (`KismetSystemLibrary.PrintString` "Win !" true true (struct :`R` 0.027518 :`G` 1.0 :`B` 0.003077 :`A` 1.0))
          (bind _returnvalue_4 (`GameplayStatics.GetActorOfClass` "/Script/Engine.CameraActor"))
          (`PlayerController.SetViewTargetWithBlend` _returnvalue_3 _returnvalue_4 0.5 "VTBlend_EaseOut" 0.0 false)
          (bind _returnvalue_5 (`|CreateWidget` "/Game/Widgets/WBP_GameOverScreen.WBP_GameOverScreen_C" _returnvalue_3))
          (`/Game/Widgets/WBP_GameOverScreen.UpdateGameResultText` _returnvalue_5 "Victory :D" (struct :`R` 0.11552 :`G` 1.0 :`B` 0.017854 :`A` 1.0))
          (`UserWidget.AddToViewport` _returnvalue_5 0))
        (:`NewEnumerator1`
          (`KismetSystemLibrary.PrintString` "Lose!" true true (struct :`R` 1.0 :`G` 0.01861 :`A` 1.0))
          (`/Game/ThirdPerson/Blueprints/BP_ThirdPersonCharacter.Death` _asbp_third_person_character)
          (`SceneComponent.K2_DetachFromComponent` (`/Game/ThirdPerson/Blueprints/BP_ThirdPersonCharacter.FollowCamera` _asbp_third_person_character) "KeepWorld" "KeepWorld" "KeepWorld" true)
          (`PlayerController.SetViewTargetWithBlend` _returnvalue_2 null 1.0 "VTBlend_Linear" 0.0 false)
          (`GameplayStatics.PlaySoundAtLocation` "/Game/StarterContent/Audio/jixaw-metal-pipe-falling-sound.jixaw-metal-pipe-falling-sound" (0.0 0.0 0.0) (struct) 1.0 1.0 0.0 null null null null)
          (bind _returnvalue_6 (`|CreateWidget` "/Game/Widgets/WBP_GameOverScreen.WBP_GameOverScreen_C" _returnvalue_2))
          (`/Game/Widgets/WBP_GameOverScreen.UpdateGameResultText` _returnvalue_6 "Skill Issue :P" (struct :`R` 1.0 :`G` 0.025338 :`B` 0.028388 :`A` 1.0))
          (`UserWidget.AddToViewport` _returnvalue_6 0))))))

(fn `UserConstructionScript`)